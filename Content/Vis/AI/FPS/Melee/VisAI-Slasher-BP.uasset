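; Slasher melee AI character on the VisAI framework that grows more aggressive as it loses health.
; Damage restarts its behavior tree as Passive, Murderous or Psychotic by health threshold, plays hit reactions and ragdolls it at zero health.
; MeleeSphere overlaps set attack or, at lower health, stab flags on authority, while MeleeAttack and StabAttack damage overlapping controller targets.
; Key bindings feed prioritized GrappleComponent attempts and toggle slow motion, alongside debug prints.
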(event `Change State`
  (params (State :type Byte))
  (bind _aicontrollerref (`self.AIControllerRef`))
  ;[1 1 1] Change State
  (set `self.State` State)
  (`|ExecutionSequence`
    (:`then_0`
      (`ActorComponent.K2_DestroyComponent` (`AIController.BrainComponent` _aicontrollerref)))
    (:`then_1`
      (`AIController.RunBehaviorTree` _aicontrollerref (select `byte` (`self.State`) :`0` "/Game/Vis/AI/FPS/Melee/Behaviour/01-VisAI_BT_Melee_Passive.01-VisAI_BT_Melee_Passive" :`1` "/Game/Vis/AI/FPS/Melee/Behaviour/02-VisAI_BT_Melee_Murderous.02-VisAI_BT_Melee_Murderous" :`2` "/Game/Vis/AI/FPS/Melee/Behaviour/03-VisAI_BT_Melee_Psychotic.03-VisAI_BT_Melee_Psychotic" :!type "BehaviorTree Object Reference")))))

(event `Key|CapsLock`
  (params (Key :type "Key Structure"))
  (:`Pressed`
    (`/Engine/EditorBlueprintResources/StandardMacros.FlipFlop`
      (:`A`
        (`GameplayStatics.SetGlobalTimeDilation` 0.2))
      (:`B`
        (`GameplayStatics.SetGlobalTimeDilation` 1.0)))))

(event `Key|V`
  (params (Key :type "Key Structure"))
  ;[0.5781 0.3561 1] Input being sent over to the Grapple Component
  (:`Pressed`
    (`/GrappleComponent/GrappleComponent/GrappleComponent.Process User Command (Input)` (`self.GrappleComponent`) "PrimaryFire" "NewEnumerator1" "NewEnumerator0")))

(event `Key|G`
  (params (Key :type "Key Structure"))
  ;[1 1 1] Input actions are also processed on the parent of thes character Blueprint, so the flag 'override parent binding' on these nodes needs to be set to false.
  (:`Pressed`
    ;[0.15 0.15 0.15 1 14] This Character performs three Grapple Attempts at once. If the first one fails, the next one will be executed and so on.
    ;
    ; In this case, Grapple Objects are input in an order from 'exceptional' to 'normal'. Grapple Sequences that require special conditions to be fulfilled (eg. standing behind het arget or having two targets ate once) will have priority over the ones that don't.
    (`/GrappleComponent/GrappleComponent/GrappleComponent.Grapple Attempt Advanced (Input)` :`self` (`self.GrappleComponent`) :`Grapple Object Class` (`|MakeArray` "/Game/GrappleComponentContentExamples/SampleContent/GrappleSequence/double/G_Double.G_Double_C" "/Game/GrappleComponentContentExamples/SampleContent/GrappleSequence/stealthtakedown/G_StealthTakedown.G_StealthTakedown_C" "/Game/GrappleComponentContentExamples/SampleContent/GrappleSequence/wrestle/G_SlasherGrapple.G_SlasherGrapple_C" :!type "/GrappleComponent/GrappleComponent/StatusObject/GrappleObject Class Reference") :`Forbidden State Tags` (`|MakeArray`))))

(event `Key|G`
  (params (Key :type "Key Structure"))
  ;[0.5781 0.3561 1] Input being sent over to the Grapple Component
  (:`Pressed`
    (`/GrappleComponent/GrappleComponent/GrappleComponent.Process User Command (Input)` (`self.GrappleComponent`) "SecondaryFire" "NewEnumerator1" "NewEnumerator0")))

(event `self.ReceiveBeginPlay`
  ;[0 0 0] Begin Play
  (`parent.ReceiveBeginPlay`)
  (`|ExecutionSequence`
    (:`then_0`
      ;[0.5144 1 0.7136] Anim Reference
      (bind _asbp_martyr_anim_bp (cast `/Game/ClassicSurvivalHorrorTemplate/Blueprints/Enemies/BP_MartyrAnimBP` (`SkeletalMeshComponent.GetAnimInstance` (`self.Mesh`))))
      (set `self.AnimReference` _asbp_martyr_anim_bp))
    (:`then_1`
      (set `/Game/Vis/BP/HealthAndDamage/HealthAndDamage_C.CurrentHealth` 200.0 (`self.VisAI_HealthAndDamage_FPS`))
      (`KismetSystemLibrary.PrintString` "Health 200"))))

(event `Footstep Event`
  ;[1 1 1] Footstep Event
  (`GameplayStatics.PlaySoundAtLocation` "/Game/ClassicSurvivalHorrorTemplate/Audio/SFX/Cue/NormalFootstep4_Cue.NormalFootstep4_Cue" (`self.K2_GetActorLocation`) (struct) 1.0 1.0 0.0 null null null))

(event `End Stab`
  ;[0 0 0] Melee Attack
  ;;[0.375 0.375 0.375] End Attack
  (set `self.isStabbing` false))

(event `Begin Stab`
  ;[0 0 0] Melee Attack
  ;;[0.4427 0.4427 0.4427] Begin Attack
  (if (not (`/Game/Vis/BP/HealthAndDamage/HealthAndDamage_C.IsDead` (`self.VisAI_HealthAndDamage_FPS`)))
    (set `self.isStabbing` true)))

(event `Begin Attack`
  ;[0 0 0] Melee Attack
  ;;[0.4427 0.4427 0.4427] Begin Attack
  (if (not (`/Game/Vis/BP/HealthAndDamage/HealthAndDamage_C.IsDead` (`self.VisAI_HealthAndDamage_FPS`)))
    (set `self.IsAttacking` true)))

(event `End Attack`
  ;[0 0 0] Melee Attack
  ;;[0.375 0.375 0.375] End Attack
  (set `self.IsAttacking` false))

(event `self.ReceiveAnyDamage`
  (params (Damage :type "Float (single-precision)") (DamageType :type "DamageType Object Reference") (InstigatedBy :type "Controller Object Reference") (DamageCauser :type "Actor Object Reference"))
  (bind _mesh (`self.Mesh`))
  ;[0 0 0] Melee Attack
  ;;[0.349 0.349 0.349] Try begin attack on damaged
  (`|ExecutionSequence`
    (:`then_0`
      (if (<= (`/Game/Vis/BP/HealthAndDamage/HealthAndDamage_C.CurrentHealth` (`self.VisAI_HealthAndDamage_FPS`)) 133.0)
        (`self.Change State` 1)
        (`KismetSystemLibrary.PrintString` "Murderous-BT" true true (struct :`G` 0.66 :`B` 1.0 :`A` 1.0) 10.0)
        (if (<= (`/Game/Vis/BP/HealthAndDamage/HealthAndDamage_C.CurrentHealth` (`self.VisAI_HealthAndDamage_FPS`)) 66.0)
          (`self.Change State` 2)
          (`KismetSystemLibrary.PrintString` "PSYCHO-BT" true true (struct :`G` 0.66 :`B` 1.0 :`A` 1.0) 10.0)
          (else
            (`self.Change State` 1)
            (`KismetSystemLibrary.PrintString` "Murderous-BT" true true (struct :`G` 0.66 :`B` 1.0 :`A` 1.0) 10.0)))
        (else
          (`self.Change State` 0)
          (`KismetSystemLibrary.PrintString` "Passive-BT" true true (struct :`G` 0.66 :`B` 1.0 :`A` 1.0) 10.0))))
    (:`then_1`
      (`KismetSystemLibrary.PrintText` (`KismetTextLibrary.Conv_DoubleToText` Damage "HalfToEven"))
      (if (<= (`/Game/Vis/BP/HealthAndDamage/HealthAndDamage_C.GetCurrentHealthPercentage` (`self.VisAI_HealthAndDamage_FPS`)) 0.0)
        ;;;[1 1 1] Initialize ragdoll
        (`SkeletalMeshComponent.SetAllBodiesBelowSimulatePhysics` _mesh (`SkinnedMeshComponent.GetBoneName` _mesh 0) true true)
        ;;;[1 1 1] Disable Collision
        (`PrimitiveComponent.SetCollisionEnabled` (`self.CapsuleComponent`) "NoCollision")
        (`PrimitiveComponent.SetCollisionEnabled` (`self.SM_Knife`) "NoCollision")
        (`PrimitiveComponent.SetCollisionEnabled` (`self.MeleeSphere`) "NoCollision")
        (`PrimitiveComponent.SetCollisionEnabled` (`self.Robe-Tail`) "NoCollision")
        (`ActorComponent.Deactivate` (`self.AIPerceptionStimuliSource`))
        (`CharacterMovementComponent.DisableMovement` (`self.CharacterMovement`))
        (else
          (`self.AI-HitReaction`)
          (if (`self.ShouldBeginAttack` DamageCauser)
            _))))))

(event `self.MeleeSphere.OnComponentBeginOverlap`
  (params (OverlappedComponent :type "PrimitiveComponent Object Reference") (OtherActor :type "Actor Object Reference") (OtherComp :type "PrimitiveComponent Object Reference") (OtherBodyIndex :type Integer) (bFromSweep :type Boolean) (SweepResult :type "HitResult Structure (by ref)"))
  ;[0 0 0] Melee Attack
  ;;[0.02951 0.02951 0.02951] Set and clear attack timer by overlap
  (if (`self.ShouldBeginAttack` OtherActor)
    (`/Engine/EditorBlueprintResources/ActorMacros.Switch Has Authority`
      (:`Authority`
        (if (<= (`/Game/Vis/BP/HealthAndDamage/HealthAndDamage_C.CurrentHealth` (`self.VisAI_HealthAndDamage_FPS`)) 133.0)
          (`self.Begin Stab`)
          (else
            (`self.Begin Attack`)))))))

(event `self.MeleeSphere.OnComponentEndOverlap`
  (params (OverlappedComponent :type "PrimitiveComponent Object Reference") (OtherActor :type "Actor Object Reference") (OtherComp :type "PrimitiveComponent Object Reference") (OtherBodyIndex :type Integer))
  ;[0 0 0] Melee Attack
  ;;[0.02951 0.02951 0.02951] Set and clear attack timer by overlap
  (if (`self.ShouldEndAttack` OtherActor)
    (`/Engine/EditorBlueprintResources/ActorMacros.Switch Has Authority`
      (:`Authority`
        (if (<= (`/Game/Vis/BP/HealthAndDamage/HealthAndDamage_C.CurrentHealth` (`self.VisAI_HealthAndDamage_FPS`)) 133.0)
          (`self.End Stab`)
          (else
            (`self.End Attack`)))))))

(fn `AI-HitReaction`
  (bind _returnvalue (`self.K2_GetActorLocation`))
  (`KismetSystemLibrary.PrintString` "Ouch1")
  (if (`/Game/Vis/BP/HealthAndDamage/HealthAndDamage_C.IsDead` (`self.VisAI_HealthAndDamage_FPS`))
    (`KismetSystemLibrary.PrintString` "Ouch-A")
    (`/Engine/EditorBlueprintResources/StandardMacros.DoOnce` false
      (:`Completed`
        (`GameplayStatics.PlaySoundAtLocation` "/Game/ClassicSurvivalHorrorTemplate/Audio/SFX/Cue/ReceiveDamage1_Cue.ReceiveDamage1_Cue" _returnvalue (struct) 1.0 1.0 0.0 null null null)))
    (else
      (`KismetSystemLibrary.PrintString` "Ouch-B")
      (bind _asbp_slasher_mixamo_anim_bp (cast `/Game/ClassicSurvivalHorrorTemplate/Blueprints/Player/BP_SlasherMixamoAnimBP` (`SkeletalMeshComponent.GetAnimInstance` (`self.Mesh`))))
      (set `/Game/ClassicSurvivalHorrorTemplate/Blueprints/Player/BP_SlasherMixamoAnimBP.Damaged?` true _asbp_slasher_mixamo_anim_bp)
      (`GameplayStatics.PlaySoundAtLocation` "/Game/ClassicSurvivalHorrorTemplate/Audio/SFX/Cue/MonsterSound_Cue.MonsterSound_Cue" _returnvalue (struct) 1.0 1.0 0.0 null null null)))
  ;[1 1 1] Blood Particle
  (`GameplayStatics.SpawnEmitterAtLocation` "/Game/ClassicSurvivalHorrorTemplate/Particles/BloodSplatter_Particle.BloodSplatter_Particle" _returnvalue)
  (`KismetSystemLibrary.PrintString` "Ouch2"))

(fn `AnyCharactersInMeleeRange`
  (returns (ReturnValue :type Boolean))
  (locals (ValidActors :type "Array of Actor Object Reference"))
  (`KismetArrayLibrary.Array_Clear` (`local.ValidActors`))
  (for _array_element (`PrimitiveComponent.GetOverlappingActors` (`self.MeleeSphere`) "/Script/Engine.Character")
    (if (`self.Enemy Check` _array_element)
      (`KismetArrayLibrary.Array_Add` (`local.ValidActors`) _array_element)))
  (return (> (`KismetArrayLibrary.Array_Length` (`local.ValidActors`)) 0)))

(fn `Enemy Check`
  (params (Actor :type "Actor Object Reference"))
  (returns (return :type Boolean))
  (locals (TempBool :type Boolean))
  (bind (_valid _visai_controller) (`/Game/Vis/AI/Base/Parent/VisAI_FunctionLibrary.Get Owning VisAI Controller From Pawn` self))
  ;[0.09549 0.09549 0.09549] Valid?
  (`/Engine/EditorBlueprintResources/StandardMacros.IsValid` Actor
    (:`Is Valid`
      ;[0.09549 0.09549 0.09549] Not self?
      (if (!= Actor self)
        ;[0.09549 0.09549 0.09549] Not owned by self
        (if (!= (`self.GetOwner` Actor) self)
          ;[0.09549 0.09549 0.09549] Are they a target?
          (if _valid
            (`/Engine/EditorBlueprintResources/StandardMacros.IsValid` _visai_controller
              (:`Is Valid`
                (set `local.TempBool` (`/Game/Vis/AI/Base/Parent/VisAI_Controller.IsActorTarget` _visai_controller Actor))
                ;[0.09549 0.09549 0.09549] tempbool is here cus bugs
                (return (`local.TempBool`)))
              (:`Is Not Valid`
                _))))))
    (:`Is Not Valid`
      _))
  (return false))

(fn `FootstepSound`
  (`GameplayStatics.PlaySoundAtLocation` "/Game/ClassicSurvivalHorrorTemplate/Audio/SFX/Cue/NormalFootstep4_Cue.NormalFootstep4_Cue" (`self.K2_GetActorLocation`) (struct) 1.0 1.0 0.0 null null null))

(fn `MeleeAttack`
  (locals (OverlappingActors :type "Array of Actor Object Reference"))
  (`KismetSystemLibrary.PrintString` "Ambyyyy?")
  ;[0.09549 0.09549 0.09549] Are there any Characters in melee range?
  (if (`self.AnyCharactersInMeleeRange`)
    ;[0.09549 0.09549 0.09549] Yes, add them for reference
    (`KismetSystemLibrary.PrintString` "yES Amby")
    (bind _output_get (set `local.OverlappingActors` (`PrimitiveComponent.GetOverlappingActors` (`self.MeleeSphere`) "/Script/Engine.Character")))
    ;[0.09549 0.09549 0.09549] Loop through and apply damage
    (for _array_element _output_get
      ;;[0.36 0.36 0.36] Are they an enemy?
      (if (`self.Enemy Check` _array_element)
        (`GameplayStatics.ApplyDamage` _array_element (`self.MeleeDamage`) null self)
        (`KismetSystemLibrary.PrintString` "Apply Damage")))
    (else
      (`/Engine/EditorBlueprintResources/ActorMacros.Switch Has Authority`
        (:`Authority`
          ;[0.09549 0.09549 0.09549] End Attack
          (`self.End Attack`))
        (:`Remote`)))))

(fn `ReceiveDamage`
  (params (HitResult :type "HitResult Structure"))
  (`GameplayStatics.ApplyDamage` (`.HitActor` (`GameplayStatics.BreakHitResult` HitResult)) 20.0)
  (set `self.isDamaged` true)
  (`self.AI-HitReaction`)
  (`KismetSystemLibrary.PrintString` "Received Damage"))

(fn `ShouldBeginAttack`
  (params (`Actor To Damage` :type "Actor Object Reference"))
  (returns (return :type Boolean))
  (return (and (`self.Enemy Check` `Actor To Damage`) (not (`self.IsAttacking`)))))

(fn `ShouldEndAttack`
  (params (Actor :type "Actor Object Reference"))
  (returns (return :type Boolean))
  (return (and (`self.Enemy Check` Actor) (not (`self.AnyCharactersInMeleeRange`)))))

(fn `StabAttack`
  (locals (OverlappingActors :type "Array of Actor Object Reference"))
  (`KismetSystemLibrary.PrintString` "Ambyyyy?")
  ;[0.09549 0.09549 0.09549] Are there any Characters in melee range?
  (if (`self.AnyCharactersInMeleeRange`)
    ;[0.09549 0.09549 0.09549] Yes, add them for reference
    (`KismetSystemLibrary.PrintString` "yES Amby")
    (bind _output_get (set `local.OverlappingActors` (`PrimitiveComponent.GetOverlappingActors` (`self.MeleeSphere`) "/Script/Engine.Character")))
    ;[0.09549 0.09549 0.09549] Loop through and apply damage
    (for _array_element _output_get
      ;;[0.36 0.36 0.36] Are they an enemy?
      (if (`self.Enemy Check` _array_element)
        (`GameplayStatics.ApplyDamage` _array_element (`self.MeleeDamage`) null self)
        (`KismetSystemLibrary.PrintString` "Apply Damage")))
    (else
      (`/Engine/EditorBlueprintResources/ActorMacros.Switch Has Authority`
        (:`Authority`
          ;[0.09549 0.09549 0.09549] End Attack
          (`self.End Stab`))
        (:`Remote`)))))

(fn `UserConstructionScript`
  (`parent.UserConstructionScript`))