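; BP_PickupDocument is a world pickup that gives the player a document in a survival horror game.
; A box overlap stores the player-tagged actor and enables input only while they are in range, and a looping delay re-triggers a shine effect.
; Pressing Action once sends the document data and an "obtained" notification to the player, plays a sound, then destroys the actor.
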(event `self.ReceiveBeginPlay`
  ;[1 1 1] Event BeginPlay
  ;[1 1 1] Loop (Shining)
  (`ActorComponent.Activate` (`self.Shining`) true :!label _label)
  (`KismetSystemLibrary.Delay` 3.0)
  (goto _label))

(event `self.Box.OnComponentBeginOverlap`
  (params (OverlappedComponent :type "PrimitiveComponent Object Reference") (OtherActor :type "Actor Object Reference") (OtherComp :type "PrimitiveComponent Object Reference") (OtherBodyIndex :type Integer) (bFromSweep :type Boolean) (SweepResult :type "HitResult Structure (by ref)"))
  ;[1 1 1] Overlap Detect
  (if (`self.ActorHasTag` OtherActor "Player")
    (set `self.PlayerActor` OtherActor)
    (`self.EnableInput` (`GameplayStatics.GetPlayerController` 0))))

(event `InputAction|Action`
  (params (Key :type "Key Structure"))
  (bind _f_document_name (break `/Game/ClassicSurvivalHorrorTemplate/Blueprints/Player/S_DocumentInfo` (`self.F_Document`)))
  ;[1 1 1] Action - Pickup
  (:`Pressed`
    (`/Engine/EditorBlueprintResources/StandardMacros.DoOnce` false
      (:`Completed`
        (message `/Game/ClassicSurvivalHorrorTemplate/Blueprints/Player/PlayerInterface.PickupDocument` (`self.PlayerActor`) (`self.F_Document`))
        (`GameplayStatics.PlaySound2D` (`self.PickupSound`) 1.0 1.0 0.0 null null)
        (`self.ObtainedItemNotification` _f_document_name " obtained")
        (`self.K2_DestroyActor`)))))

(event `self.Box.OnComponentEndOverlap`
  (params (OverlappedComponent :type "PrimitiveComponent Object Reference") (OtherActor :type "Actor Object Reference") (OtherComp :type "PrimitiveComponent Object Reference") (OtherBodyIndex :type Integer))
  ;[1 1 1] Overlap Detect
  (if (`self.ActorHasTag` OtherActor "Player")
    (set `self.PlayerActor` null)
    (`self.DisableInput` (`GameplayStatics.GetPlayerController` 0))))

(fn `ObtainedItemNotification`
  (params (A :type String) (B :type String) (`Addon(Optional)` :type String))
  (message `/Game/ClassicSurvivalHorrorTemplate/Blueprints/Player/PlayerInterface.Notification` (`self.PlayerActor`) A B `Addon(Optional)`))

(fn `UserConstructionScript`)