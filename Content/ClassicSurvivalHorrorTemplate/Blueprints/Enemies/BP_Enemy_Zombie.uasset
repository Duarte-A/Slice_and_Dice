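; Zombie enemy for a survival horror game that chases a seen player and attacks at close range.
; Pawn sensing drives AI movement, while a box overlap toggles the attack flag on its animation Blueprint.
; The attack event multi-sphere traces forward from the neck socket, applying damage, blood and sound to hits.
; Hit reactions spawn blood and either flag damage on the animation or, when dead, play a one-time death sound.
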(event `self.ReceiveBeginPlay`
  ;[1 1 1] Event Begin Play
  (`|ExecutionSequence`
    (:`then_0`
      ;[0.5144 1 0.7136] Anim Reference
      (bind _asbp_zombie_anim_bp (cast `/Game/ClassicSurvivalHorrorTemplate/Blueprints/Enemies/BP_ZombieAnimBP` (`SkeletalMeshComponent.GetAnimInstance` (`self.Mesh`))))
      (set `self.AnimReference` _asbp_zombie_anim_bp))))

(event `self.Box.OnComponentBeginOverlap`
  (params (OverlappedComponent :type "PrimitiveComponent Object Reference") (OtherActor :type "Actor Object Reference") (OtherComp :type "PrimitiveComponent Object Reference") (OtherBodyIndex :type Integer) (bFromSweep :type Boolean) (SweepResult :type "HitResult Structure (by ref)"))
  ;[1 0.6269 0.3385] Overlapping Player
  (if (`self.ActorHasTag` OtherActor "Player")
    ;[1 0.7518 0.3458] Attack when near
    (set `/Game/ClassicSurvivalHorrorTemplate/Blueprints/Enemies/BP_ZombieAnimBP.Attacking?` true (`self.AnimReference`))))

(event `self.PawnSensing.OnSeePawn`
  (params (Pawn :type "Pawn Object Reference"))
  ;[0.8096 1 0.2572] Chase Player
  (`|AIMoveTo` self (0.0 0.0 0.0) Pawn))

(event `self.Box.OnComponentEndOverlap`
  (params (OverlappedComponent :type "PrimitiveComponent Object Reference") (OtherActor :type "Actor Object Reference") (OtherComp :type "PrimitiveComponent Object Reference") (OtherBodyIndex :type Integer))
  ;[1 0.6269 0.3385] Overlapping Player
  (if (`self.ActorHasTag` OtherActor "Player")
    ;[1 0.7518 0.3458] Don't attack when far
    (set `/Game/ClassicSurvivalHorrorTemplate/Blueprints/Enemies/BP_ZombieAnimBP.Attacking?` false (`self.AnimReference`))))

(event `Attack_1`
  (bind _returnvalue (`SceneComponent.GetSocketLocation` (`self.Mesh`) "Neck"))
  ;[1 0.2488 0.2289] Deal damage during animation
  (if (not (`self.Dead`))
    ;[1 0.3842 0.2339] Multisphere Trace
    (bind (_outhits _returnvalue_2) (`KismetSystemLibrary.SphereTraceMulti` _returnvalue (+ _returnvalue (* (`KismetMathLibrary.GetForwardVector` (`self.K2_GetActorRotation`)) 90.0)) 50.0 "TraceTypeQuery1"))
    (if _returnvalue_2
      (for _array_element _outhits
        (bind (_bblockinghit _binitialoverlap _time _distance _location _impactpoint _normal _impactnormal _physmat _hitactor) (`GameplayStatics.BreakHitResult` _array_element))
        (`GameplayStatics.ApplyDamage` _hitactor 20.0)
        ;[1 1 1] Blood Splatter
        (`GameplayStatics.SpawnEmitterAtLocation` "/Game/ClassicSurvivalHorrorTemplate/Particles/BloodSplatter_Particle.BloodSplatter_Particle" _impactpoint)
        ;[1 1 1] Play Monster Sound
        (`GameplayStatics.PlaySoundAtLocation` "/Game/ClassicSurvivalHorrorTemplate/Audio/SFX/Cue/MonsterSound_Cue.MonsterSound_Cue" (`self.K2_GetActorLocation`) (struct) 1.0 1.0 0.0 null null null)))))

(event `HitReaction_1`
  (bind _returnvalue (`self.K2_GetActorLocation`))
  ;[1 1 1] Hit Reaction
  (if (`self.Dead`)
    (`/Engine/EditorBlueprintResources/StandardMacros.DoOnce` false
      (:`Completed`
        (`GameplayStatics.PlaySoundAtLocation` "/Game/ClassicSurvivalHorrorTemplate/Audio/SFX/Cue/MonsterDeath_Cue.MonsterDeath_Cue" _returnvalue (struct) 1.0 1.0 0.0 null null null)))
    (else
      (set `/Game/ClassicSurvivalHorrorTemplate/Blueprints/Enemies/BP_ZombieAnimBP.Damaged?` true (`self.AnimReference`))
      (`GameplayStatics.PlaySoundAtLocation` "/Game/ClassicSurvivalHorrorTemplate/Audio/SFX/Cue/MonsterSound_Cue.MonsterSound_Cue" _returnvalue (struct) 1.0 1.0 0.0 null null null)))
  ;;[1 1 1] Blood Particle
  (`GameplayStatics.SpawnEmitterAtLocation` "/Game/ClassicSurvivalHorrorTemplate/Particles/BloodSplatter_Particle.BloodSplatter_Particle" _returnvalue))

(fn `UserConstructionScript`
  (`parent.UserConstructionScript`))