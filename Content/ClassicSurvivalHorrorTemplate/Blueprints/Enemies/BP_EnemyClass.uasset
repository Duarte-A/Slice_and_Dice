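; Enemy class for the survival horror template that handles taking damage and dying.
; AnyDamage subtracts from HP and, at zero or below, ragdolls the mesh from the root bone, flags Dead and disables capsule collision.
; KillAnimations freezes the mesh's global animation rate during ragdoll by inverting a bool into a rate scale.
; Death also clears SensedEnemy on player zero, supporting both Mixamo and UE4 Mannequin player Blueprints.
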(event `self.ReceiveAnyDamage`
  (params (Damage :type "Float (single-precision)") (DamageType :type "DamageType Object Reference") (InstigatedBy :type "Controller Object Reference") (DamageCauser :type "Actor Object Reference"))
  (bind _mesh (`self.Mesh`))
  ;[1 0.4375 0.4375] Event AnyDamage
  (bind _output_get (set `self.HP` (- (`self.HP`) Damage)))
  (if (<= _output_get 0.0)
    ;[1 1 1] Initialize ragdoll
    (`SkeletalMeshComponent.SetAllBodiesBelowSimulatePhysics` _mesh (`SkinnedMeshComponent.GetBoneName` _mesh 0) true true)
    ;[1 1 1] Dead = TRUE
    (set `self.Dead` true)
    ;[1 1 1] Capsule Collision = FALSE
    (`PrimitiveComponent.SetCollisionEnabled` (`self.CapsuleComponent`) "NoCollision")
    ;[1 1 1] Prevent animations from playing while in ragdoll
    (`self.KillAnimations` true)
    (`|ExecutionSequence`
      (:`then_0`
        ;[1 0.103 0.0831] Nullify Targetted Enemy (Mixamo)
        (bind _asbp_mixamo_player (cast `/Game/ClassicSurvivalHorrorTemplate/Blueprints/Player/BP_MixamoPlayer` (`GameplayStatics.GetPlayerPawn` 0)))
        (set `/Game/ClassicSurvivalHorrorTemplate/Blueprints/Player/BP_MixamoPlayer.SensedEnemy` null _asbp_mixamo_player))
      (:`then_1`
        ;[0.202 0.2814 1] Nullify Targetted Enemy (UE4 Mannequin)
        (bind _asbp_ue4player (cast `/Game/ClassicSurvivalHorrorTemplate/Blueprints/Player/BP_UE4Player` (`GameplayStatics.GetPlayerPawn` 0)))
        (set `/Game/ClassicSurvivalHorrorTemplate/Blueprints/Player/BP_UE4Player.SensedEnemy` null _asbp_ue4player)))))

(fn `KillAnimations`
  (params (Stop :type Boolean))
  (set `SkeletalMeshComponent.GlobalAnimRateScale` (* (- (`KismetMathLibrary.Conv_BoolToDouble` Stop) 1.0) -1.0) (`self.Mesh`)))

(fn `UserConstructionScript`)