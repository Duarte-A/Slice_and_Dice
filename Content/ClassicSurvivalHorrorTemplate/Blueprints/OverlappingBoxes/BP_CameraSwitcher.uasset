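; Trigger box that switches the player's view to its assigned camera for fixed-camera survival horror framing.
; Player-tagged overlaps, the SwitchCamera event, or a one-time Tick check for a player already inside the box set the view target.
; Each switch messages the overlapping actor, or the player character as fallback, with the latest camera and whether it is rotatable.
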(event `self.ReceiveTick`
  (params (DeltaSeconds :type "Float (single-precision)"))
  (bind _rotatablecamera_ (`self.RotatableCamera?`))
  (bind _cameraactor (`self.CameraActor`))
  ;[1 1 1] Initializing Camera Switching
  (if (`PrimitiveComponent.IsOverlappingActor` (`self.Box`) (`GameplayStatics.GetPlayerCharacter` 0))
    (`/Engine/EditorBlueprintResources/StandardMacros.DoOnce` false
      (:`Completed`
        ;[1 1 1] Switch to new camera after overlap
        (`PlayerController.SetViewTargetWithBlend` (`GameplayStatics.GetPlayerController` 0) _cameraactor 0.0 "VTBlend_Linear" 0.0 false :!label _label)
        (`/Engine/EditorBlueprintResources/StandardMacros.IsValid` (stale `self.Box.OnComponentBeginOverlap` OtherActor)
          (:`Is Valid`
            ;[1 1 1] Save as latest camera & prepare for current used camera
            (message `/Game/ClassicSurvivalHorrorTemplate/Blueprints/Player/PlayerInterface.SwitchCamera` (stale `self.Box.OnComponentBeginOverlap` OtherActor) _cameraactor _rotatablecamera_))
          (:`Is Not Valid`
            (message `/Game/ClassicSurvivalHorrorTemplate/Blueprints/Player/PlayerInterface.SwitchCamera` (`GameplayStatics.GetPlayerCharacter` 0) _cameraactor _rotatablecamera_)))))))

(event `self.Box.OnComponentBeginOverlap`
  (params (OverlappedComponent :type "PrimitiveComponent Object Reference") (OtherActor :type "Actor Object Reference") (OtherComp :type "PrimitiveComponent Object Reference") (OtherBodyIndex :type Integer) (bFromSweep :type Boolean) (SweepResult :type "HitResult Structure (by ref)"))
  ;[1 1 1] Switch to new camera after overlap
  (if (`self.ActorHasTag` OtherActor "Player")
    (goto _label)))

(event `SwitchCamera`
  ;[1 1 1] Switch to new camera after overlap
  (goto _label))

(fn `UserConstructionScript`)