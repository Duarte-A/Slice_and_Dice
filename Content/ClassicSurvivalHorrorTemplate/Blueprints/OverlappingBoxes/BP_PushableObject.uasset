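; Pushable heavy object that the player shoves along the world X or Y axis by pressing Action beside it.
; Four side overlap boxes detect the Player-tagged actor, record the push direction in BoxFocused and toggle input on the actor.
; The matching timeline nudges the mesh each update with a swept move.
; A DoOnce plays the push sound and sets a Pushing lock, both reset when the timeline finishes.
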(event `InputAction|Action`
  (params (Key :type "Key Structure"))
  (bind _mesh (`self.Mesh`))
  (bind (_returnvalue_x _returnvalue_y _returnvalue_z) (`KismetMathLibrary.BreakVector` (`SceneComponent.K2_GetComponentLocation` (`self.Mesh`))))
  ;[1 1 1] Action - Push Object
  (:`Pressed`
    (if (not (`self.Pushing?`))
      (switch `int` (`self.BoxFocused`)
        (:`1`
          (bind (_direction _alpha) (`Timeline|Timeline_0` :!via `PlayFromStart`)
            (:`Update`
              (`SceneComponent.K2_SetWorldLocation` _mesh (`KismetMathLibrary.MakeVector` _returnvalue_x (- _returnvalue_y (`KismetMathLibrary.Lerp` 0.0 3.0 _alpha)) _returnvalue_z) true false)
              (`/Engine/EditorBlueprintResources/StandardMacros.DoOnce` false :!label _label
                (:`Completed`
                  (`GameplayStatics.PlaySoundAtLocation` "/Game/ClassicSurvivalHorrorTemplate/Audio/SFX/Cue/PushHeavyObject_Cue.PushHeavyObject_Cue" (`SceneComponent.K2_GetComponentLocation` (`self.Mesh`)) (struct) 1.0 1.0 0.0 null null null)
                  (set `self.Pushing?` true))))
            (:`Finished`
              (set `self.Pushing?` false :!label _label_2)
              (`self.ResetFunctionality`))))
        (:`2`
          (bind (_direction_2 _alpha_2) (`Timeline|Timeline_1` :!via `PlayFromStart`)
            (:`Update`
              (`SceneComponent.K2_SetWorldLocation` _mesh (`KismetMathLibrary.MakeVector` _returnvalue_x (+ _returnvalue_y (`KismetMathLibrary.Lerp` 0.0 3.0 _alpha_2)) _returnvalue_z) true false)
              (goto _label))
            (:`Finished`
              (goto _label_2))))
        (:`3`
          (bind (_direction_3 _alpha_3) (`Timeline|Timeline_2` :!via `PlayFromStart`)
            (:`Update`
              (`SceneComponent.K2_SetWorldLocation` _mesh (`KismetMathLibrary.MakeVector` (- _returnvalue_x (`KismetMathLibrary.Lerp` 0.0 3.0 _alpha_3)) _returnvalue_y _returnvalue_z) true false)
              (goto _label))
            (:`Finished`
              (goto _label_2))))
        (:`4`
          (bind (_direction_4 _alpha_4) (`Timeline|Timeline_3` :!via `PlayFromStart`)
            (:`Update`
              (`SceneComponent.K2_SetWorldLocation` _mesh (`KismetMathLibrary.MakeVector` (+ _returnvalue_x (`KismetMathLibrary.Lerp` 0.0 3.0 _alpha_4)) _returnvalue_y _returnvalue_z) true false)
              (goto _label))
            (:`Finished`
              (goto _label_2))))))))

(event `ResetFunctionality`
  ;[1 1 1] Action - Push Object
  (goto _label :!via `Reset`))

(event `self.BoxX+.OnComponentBeginOverlap`
  (params (OverlappedComponent :type "PrimitiveComponent Object Reference") (OtherActor :type "Actor Object Reference") (OtherComp :type "PrimitiveComponent Object Reference") (OtherBodyIndex :type Integer) (bFromSweep :type Boolean) (SweepResult :type "HitResult Structure (by ref)"))
  ;[1 1 1] Overlap On
  (if (`self.ActorHasTag` OtherActor "Player")
    (set `self.BoxFocused` 4)
    (`self.EnableInput` (`GameplayStatics.GetPlayerController` 0))))

(event `self.BoxY-.OnComponentBeginOverlap`
  (params (OverlappedComponent :type "PrimitiveComponent Object Reference") (OtherActor :type "Actor Object Reference") (OtherComp :type "PrimitiveComponent Object Reference") (OtherBodyIndex :type Integer) (bFromSweep :type Boolean) (SweepResult :type "HitResult Structure (by ref)"))
  ;[1 1 1] Overlap On
  (if (`self.ActorHasTag` OtherActor "Player")
    (set `self.BoxFocused` 1)
    (`self.EnableInput` (`GameplayStatics.GetPlayerController` 0))))

(event `self.BoxX-.OnComponentBeginOverlap`
  (params (OverlappedComponent :type "PrimitiveComponent Object Reference") (OtherActor :type "Actor Object Reference") (OtherComp :type "PrimitiveComponent Object Reference") (OtherBodyIndex :type Integer) (bFromSweep :type Boolean) (SweepResult :type "HitResult Structure (by ref)"))
  ;[1 1 1] Overlap On
  (if (`self.ActorHasTag` OtherActor "Player")
    (set `self.BoxFocused` 3)
    (`self.EnableInput` (`GameplayStatics.GetPlayerController` 0))))

(event `self.BoxY+.OnComponentBeginOverlap`
  (params (OverlappedComponent :type "PrimitiveComponent Object Reference") (OtherActor :type "Actor Object Reference") (OtherComp :type "PrimitiveComponent Object Reference") (OtherBodyIndex :type Integer) (bFromSweep :type Boolean) (SweepResult :type "HitResult Structure (by ref)"))
  ;[1 1 1] Overlap On
  (if (`self.ActorHasTag` OtherActor "Player")
    (set `self.BoxFocused` 2)
    (`self.EnableInput` (`GameplayStatics.GetPlayerController` 0))))

(event `self.BoxY+.OnComponentEndOverlap`
  (params (OverlappedComponent :type "PrimitiveComponent Object Reference") (OtherActor :type "Actor Object Reference") (OtherComp :type "PrimitiveComponent Object Reference") (OtherBodyIndex :type Integer))
  ;[1 1 1] Overlap Off
  (if (`self.ActorHasTag` OtherActor "Player")
    (set `self.BoxFocused` 0)
    (`self.DisableInput` (`GameplayStatics.GetPlayerController` 0))))

(event `self.BoxX-.OnComponentEndOverlap`
  (params (OverlappedComponent :type "PrimitiveComponent Object Reference") (OtherActor :type "Actor Object Reference") (OtherComp :type "PrimitiveComponent Object Reference") (OtherBodyIndex :type Integer))
  ;[1 1 1] Overlap Off
  (if (`self.ActorHasTag` OtherActor "Player")
    (set `self.BoxFocused` 0)
    (`self.DisableInput` (`GameplayStatics.GetPlayerController` 0))))

(event `self.BoxY-.OnComponentEndOverlap`
  (params (OverlappedComponent :type "PrimitiveComponent Object Reference") (OtherActor :type "Actor Object Reference") (OtherComp :type "PrimitiveComponent Object Reference") (OtherBodyIndex :type Integer))
  ;[1 1 1] Overlap Off
  (if (`self.ActorHasTag` OtherActor "Player")
    (set `self.BoxFocused` 0)
    (`self.DisableInput` (`GameplayStatics.GetPlayerController` 0))))

(event `self.BoxX+.OnComponentEndOverlap`
  (params (OverlappedComponent :type "PrimitiveComponent Object Reference") (OtherActor :type "Actor Object Reference") (OtherComp :type "PrimitiveComponent Object Reference") (OtherBodyIndex :type Integer))
  ;[1 1 1] Overlap Off
  (if (`self.ActorHasTag` OtherActor "Player")
    (set `self.BoxFocused` 0)
    (`self.DisableInput` (`GameplayStatics.GetPlayerController` 0))))

(fn `UserConstructionScript`)