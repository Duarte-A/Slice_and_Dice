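; BP_ExaminationPlace is an overlap box that lets the player examine a spot and read up to four text comments.
; The Box enables input while an actor tagged Player overlaps it.
; Each interact press pauses the game and replaces the W_InteractionComment widget with the next comment, playing a sound on the first press only.
; A press after the configured count unpauses, removes the widget and resets the counter.
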(event `InputAction|Action` :paused true
  (params (Key :type "Key Structure"))
  ;[1 0.7956 0.6413] F - Interact
  (:`Pressed`
    (if (== (`self.CommentCount(1-4)`) (`self.CurrentCommentCount`))
      ;[0.4271 0.293 0.1455] Continue time
      (`GameplayStatics.SetGamePaused` false)
      (set `self.CurrentCommentCount` 0)
      (bind _foundwidgets (`WidgetBlueprintLibrary.GetAllWidgetsOfClass` "/Game/ClassicSurvivalHorrorTemplate/UserInterface/W_InteractionComment.W_InteractionComment_C"))
      (`Widget.RemoveFromParent` _foundwidgets)
      (else
        ;[0.4271 0.293 0.1455] Freeze time
        (`GameplayStatics.SetGamePaused` true)
        ;[0.3281 0.0913 0.07824] Clear this widget field for the incoming comment
        (bind _foundwidgets_2 (`WidgetBlueprintLibrary.GetAllWidgetsOfClass` "/Game/ClassicSurvivalHorrorTemplate/UserInterface/W_InteractionComment.W_InteractionComment_C"))
        (`Widget.RemoveFromParent` _foundwidgets_2)
        ;[1 1 1] Set current comment
        (`self.SetCurrentComment`)
        (bind _returnvalue (`|CreateWidget` "/Game/ClassicSurvivalHorrorTemplate/UserInterface/W_InteractionComment.W_InteractionComment_C"))
        ;[1 1 1] Type in how to comment
        (set `/Game/ClassicSurvivalHorrorTemplate/UserInterface/W_InteractionComment.CommentText` (`self.DisplayComment`) _returnvalue)
        (`UserWidget.AddToViewport` _returnvalue 0)
        ;[1 1 1] Counting comments
        (`self.CountLimit`)
        (`/Engine/EditorBlueprintResources/StandardMacros.DoOnce` false
          (:`Completed`
            ;[1 1 1] Add some sound if it's necessary
            (`GameplayStatics.PlaySound2D` (`self.PlaySound`) 1.0 1.0 0.0 null null)))))))

(event `self.Box.OnComponentBeginOverlap`
  (params (OverlappedComponent :type "PrimitiveComponent Object Reference") (OtherActor :type "Actor Object Reference") (OtherComp :type "PrimitiveComponent Object Reference") (OtherBodyIndex :type Integer) (bFromSweep :type Boolean) (SweepResult :type "HitResult Structure (by ref)"))
  ;[1 1 1] Enable/disable input on begin/end overlap
  (if (`self.ActorHasTag` OtherActor "Player")
    (`self.EnableInput` (`GameplayStatics.GetPlayerController` 0))))

(event `self.Box.OnComponentEndOverlap`
  (params (OverlappedComponent :type "PrimitiveComponent Object Reference") (OtherActor :type "Actor Object Reference") (OtherComp :type "PrimitiveComponent Object Reference") (OtherBodyIndex :type Integer))
  ;[1 1 1] Enable/disable input on begin/end overlap
  (if (`self.ActorHasTag` OtherActor "Player")
    (`self.DisableInput` (`GameplayStatics.GetPlayerController` 0))))

(fn `CountLimit`
  ;[1 1 1] Check if you hit count limit, if not, add to current count
  (if (not (== (`self.CommentCount(1-4)`) (`self.CurrentCommentCount`)))
    (`/Engine/EditorBlueprintResources/StandardMacros.IncrementInt` (`self.CurrentCommentCount`))))

(fn `SetCurrentComment`
  ;[0.194 0.3756 0.4271] Set comment based on current count
  (switch `int` (`self.CurrentCommentCount`)
    (:`Default`
      (set `self.DisplayComment` (`self.Comment1`) :!label _label))
    (:`0`
      (goto _label))
    (:`1`
      (set `self.DisplayComment` (`self.Comment2`)))
    (:`2`
      (set `self.DisplayComment` (`self.Comment3`)))
    (:`3`
      (set `self.DisplayComment` (`self.Comment4`)))))

(fn `UserConstructionScript`)