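; BP_TransitionActor is a two-sided door or passage that teleports the player to the opposite side behind a transition screen and sound.
; Overlapping either trigger box enables input on the actor and sets the destination to the other side's spawn point.
; Interact either transitions directly or first shows a Yes/No question widget, toggled with Next/Previous Item and optionally asked only once.
; A DoOnce guards the timed transition against repeat triggering.
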(event `InputAction|NextItem`
  (params (Key :type "Key Structure"))
  ;[0 0 0] Choose Answer
  (:`Pressed`
    (bind _foundwidgets (`WidgetBlueprintLibrary.GetAllWidgetsOfClass` "/Game/ClassicSurvivalHorrorTemplate/UserInterface/W_QuestionToProceed.W_QuestionToProceed_C"))
    (if (`KismetArrayLibrary.Array_IsValidIndex` _foundwidgets)
      (for _array_element _foundwidgets
        ;;[0 0 0] Yes
        (set `/Game/ClassicSurvivalHorrorTemplate/UserInterface/W_QuestionToProceed.AnswerNoYes` 1 _array_element)))))

(event `InputAction|PreviousItem`
  (params (Key :type "Key Structure"))
  ;[0 0 0] Choose Answer
  (:`Pressed`
    (bind _foundwidgets (`WidgetBlueprintLibrary.GetAllWidgetsOfClass` "/Game/ClassicSurvivalHorrorTemplate/UserInterface/W_QuestionToProceed.W_QuestionToProceed_C"))
    (if (`KismetArrayLibrary.Array_IsValidIndex` _foundwidgets)
      (for _array_element _foundwidgets
        ;;[0 0 0] No
        (set `/Game/ClassicSurvivalHorrorTemplate/UserInterface/W_QuestionToProceed.AnswerNoYes` 0 _array_element)))))

(event `InputAction|Action`
  (params (Key :type "Key Structure"))
  ;[1 0.789 0.6133] F - Interact
  (:`Pressed`
    (if (`self.QuestionBeforeGoing?`)
      (bind _foundwidgets (`WidgetBlueprintLibrary.GetAllWidgetsOfClass` "/Game/ClassicSurvivalHorrorTemplate/UserInterface/W_QuestionToProceed.W_QuestionToProceed_C"))
      (if (`KismetArrayLibrary.Array_IsValidIndex` _foundwidgets)
        (bind _foundwidgets_2 (`WidgetBlueprintLibrary.GetAllWidgetsOfClass` "/Game/ClassicSurvivalHorrorTemplate/UserInterface/W_QuestionToProceed.W_QuestionToProceed_C"))
        (for _array_element _foundwidgets_2
          (switch `int` (`/Game/ClassicSurvivalHorrorTemplate/UserInterface/W_QuestionToProceed.AnswerNoYes` _array_element)
            (:`0`
              ;;[0.000728 0.01042 0] Answer: No
              (bind _foundwidgets_3 (`WidgetBlueprintLibrary.GetAllWidgetsOfClass` "/Game/ClassicSurvivalHorrorTemplate/UserInterface/W_QuestionToProceed.W_QuestionToProceed_C"))
              (for _array_element_2 _foundwidgets_3
                (`Widget.RemoveFromParent` _array_element_2)))
            (:`1`
              ;;[0.000728 0.01042 0] Answer: Yes
              (bind _foundwidgets_4 (`WidgetBlueprintLibrary.GetAllWidgetsOfClass` "/Game/ClassicSurvivalHorrorTemplate/UserInterface/W_QuestionToProceed.W_QuestionToProceed_C"))
              (for _array_element_3 _foundwidgets_4
                (`Widget.RemoveFromParent` _array_element_3)
                ;;[0 0 0] Only ask once?
                (if (`self.OnlyAskOnce?`)
                  (set `self.QuestionBeforeGoing?` false))
                (`/Engine/EditorBlueprintResources/StandardMacros.DoOnce` false :!label _label
                  (:`Completed`
                    (`GameplayStatics.PlaySound2D` (`self.TransitionSound`) 1.0 1.0 0.0 null null)
                    (bind _returnvalue (`|CreateWidget` "/Game/ClassicSurvivalHorrorTemplate/UserInterface/W_TransitionScreen.W_TransitionScreen_C"))
                    (`UserWidget.AddToViewport` _returnvalue 0)
                    (`KismetSystemLibrary.Delay` 0.5)
                    (`self.K2_SetActorLocation` (`GameplayStatics.GetPlayerCharacter` 0) (`self.WhereToSpawn?`) false false)
                    (`KismetSystemLibrary.Delay` 1.0)
                    (goto _label :!via `Reset`)))))))
        (else
          ;;[0.000728 0.01042 0] Create a question
          (bind _returnvalue_2 (`|CreateWidget` "/Game/ClassicSurvivalHorrorTemplate/UserInterface/W_QuestionToProceed.W_QuestionToProceed_C"))
          (`UserWidget.AddToViewport` _returnvalue_2 0)
          (set `/Game/ClassicSurvivalHorrorTemplate/UserInterface/W_QuestionToProceed.Question` (`self.Question`) _returnvalue_2)))
      (else
        (goto _label)))))

(event `self.Box1.OnComponentBeginOverlap`
  (params (OverlappedComponent :type "PrimitiveComponent Object Reference") (OtherActor :type "Actor Object Reference") (OtherComp :type "PrimitiveComponent Object Reference") (OtherBodyIndex :type Integer) (bFromSweep :type Boolean) (SweepResult :type "HitResult Structure (by ref)"))
  ;[1 1 1] On Overlap with Box1
  (if (`self.ActorHasTag` OtherActor "Player")
    (`self.EnableInput` (`GameplayStatics.GetPlayerController` 0))
    (set `self.WhereToSpawn?` (`SceneComponent.K2_GetComponentLocation` (`self.SpawnHere2`)))))

(event `self.Box1.OnComponentEndOverlap`
  (params (OverlappedComponent :type "PrimitiveComponent Object Reference") (OtherActor :type "Actor Object Reference") (OtherComp :type "PrimitiveComponent Object Reference") (OtherBodyIndex :type Integer))
  ;[1 1 1] On Overlap with Box1
  (if (`self.ActorHasTag` OtherActor "Player")
    (`self.DisableInput` (`GameplayStatics.GetPlayerController` 0))))

(event `self.Box2.OnComponentBeginOverlap`
  (params (OverlappedComponent :type "PrimitiveComponent Object Reference") (OtherActor :type "Actor Object Reference") (OtherComp :type "PrimitiveComponent Object Reference") (OtherBodyIndex :type Integer) (bFromSweep :type Boolean) (SweepResult :type "HitResult Structure (by ref)"))
  ;[1 1 1] On Overlap with Box2
  (if (`self.ActorHasTag` OtherActor "Player")
    (`self.EnableInput` (`GameplayStatics.GetPlayerController` 0))
    (set `self.WhereToSpawn?` (`SceneComponent.K2_GetComponentLocation` (`self.SpawnHere1`)))))

(event `self.Box2.OnComponentEndOverlap`
  (params (OverlappedComponent :type "PrimitiveComponent Object Reference") (OtherActor :type "Actor Object Reference") (OtherComp :type "PrimitiveComponent Object Reference") (OtherBodyIndex :type Integer))
  ;[1 1 1] On Overlap with Box2
  (if (`self.ActorHasTag` OtherActor "Player")
    (`self.DisableInput` (`GameplayStatics.GetPlayerController` 0))))

(fn `UserConstructionScript`)